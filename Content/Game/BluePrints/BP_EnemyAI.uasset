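; Enemy character for a first-person minigame that patrols, chases the player on sight and punches on contact.
; A looping timer sends it to random navigable points around the player.
; PawnSensing pauses patrol and starts a faster, timer-driven chase, which yields back to patrol after a delay.
; A capsule hit on the player plays the punch, updates minigame state and player HP in BP_GameInstance, then opens the default level.
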(event `self.ReceiveBeginPlay`
  (bind _asbp_game_instance (cast `/Game/Game/Managers/BP_GameInstance` (`GameplayStatics.GetGameInstance`)))
  (set `self.As BP Game Instance` _asbp_game_instance)
  (bind _returnvalue (`KismetSystemLibrary.K2_SetTimerDelegate` (delegate `Patrol`) 5.0 true))
  (set `self.TimerRef` _returnvalue))

(event `Patrol`
  (set `CharacterMovementComponent.MaxWalkSpeed` 500.0 (`self.CharacterMovement`))
  (bind _randomlocation (`NavigationSystemV1.K2_GetRandomLocationInNavigableRadius` (`self.K2_GetActorLocation` (`GameplayStatics.GetPlayerCharacter` 0)) 4000.0 null null))
  (`|AIMoveTo` self _randomlocation null))

(event `self.PawnSensing.OnSeePawn`
  (params (Pawn :type "Pawn Object Reference"))
  (set `self.IsSeeingPlayer` true)
  (bind _returnvalue (`KismetSystemLibrary.K2_SetTimerDelegate` (delegate `MoveToPlayer`) 0.1 true))
  (`KismetSystemLibrary.K2_PauseTimerHandle` (`self.TimerRef`))
  (set `CharacterMovementComponent.MaxWalkSpeed` 1000.0 (`self.CharacterMovement`)))

(event `MoveToPlayer`
  (`|AIMoveTo` self (0.0 0.0 0.0) (`GameplayStatics.GetPlayerCharacter` 0)
    (:`then`
      (`/Engine/EditorBlueprintResources/StandardMacros.DoOnce` false :!label _label
        (:`Completed`
          (`KismetSystemLibrary.Delay` 3.0)
          (`|ExecutionSequence`
            (:`then_0`
              (goto _label :!via `Reset`))
            (:`then_1`
              (`KismetSystemLibrary.K2_UnPauseTimerHandle` (`self.TimerRef`))
              (set `self.IsSeeingPlayer` false)
              (`KismetSystemLibrary.K2_PauseTimerHandle` (stale `self.PawnSensing.OnSeePawn` _returnvalue)))))))))

(event `self.CapsuleComponent.OnComponentHit`
  (params (HitComponent :type "PrimitiveComponent Object Reference") (OtherActor :type "Actor Object Reference") (OtherComp :type "PrimitiveComponent Object Reference") (NormalImpulse :type "Vector Structure") (Hit :type "HitResult Structure (by ref)"))
  (bind _as_bp_game_instance (`self.As BP Game Instance`))
  (cast `/Game/Game/BluePrints/BP_FirstPersonMiniGame` OtherActor)
  (`/Engine/EditorBlueprintResources/StandardMacros.DoOnce` false
    (:`Completed`
      (`SkeletalMeshComponent.PlayAnimation` (`self.Mesh`) "/Game/Game/Characters/Anim/Mutant_Punch.Mutant_Punch" false)
      (`KismetSystemLibrary.Delay` 1.0)
      (set `/Game/Game/Managers/BP_GameInstance.MiniGameState` "NewEnumerator2" _as_bp_game_instance)
      (set `/Game/Game/Managers/BP_GameInstance.PlayerHP` (- (`/Game/Game/Managers/BP_GameInstance.PlayerHP` _as_bp_game_instance) 1) _as_bp_game_instance)
      (`GameplayStatics.OpenLevelBySoftObjectPtr` "/Game/Game/Levels/DefaultLevel.DefaultLevel"))))

(fn `UserConstructionScript`)