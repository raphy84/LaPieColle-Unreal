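; BP_Board is a board actor that holds an array of cells and provides lookup helpers for movement around them.
; On BeginPlay it casts and caches a reference to BP_GameInstance.
; GetCellByNumber returns the cell at a given index, while GetNextCellToMove wraps a cell number by the array length using modulo, so positions loop around the board.
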(event `self.ReceiveBeginPlay`
  (bind _asbp_game_instance (cast `/Game/Game/Managers/BP_GameInstance` (`GameplayStatics.GetGameInstance`)))
  (set `self.As BP Game Instance` _asbp_game_instance))

(fn `GetCellByNumber`
  (params (Number :type Integer))
  (returns (Cell :type "/Game/Game/BluePrints/Cells/BP_Cell Object Reference"))
  (return (`|GetArrayItem` (`self.Cells`) Number)))

(fn `GetNextCellToMove`
  (params (CellNumber :type Integer))
  (returns (Cell :type Integer))
  (return (mod CellNumber (`KismetArrayLibrary.Array_Length` (`self.Cells`)))))

(fn `UserConstructionScript`)