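; BP_Dice handles dice rolls that drive the movement of the Pawn and the Hunter in what appears to be a board-style game.
; On BeginPlay it creates the BPW_Main widget, adds it to the viewport and binds its dice-launch event to DiceNum.
; Each launch calls RollTheDice, which sends a six-sided roll to the Pawn's TryMoving and a separate twenty-sided roll to the Hunter's TryMovingHunter.
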(event `self.ReceiveBeginPlay`
  (bind _returnvalue (`|CreateWidget` "/Game/Game/Widget/BPW_Main.BPW_Main_C"))
  (bind _output_get (set `self.WidgetDiceRef` _returnvalue))
  (`UserWidget.AddToViewport` _output_get 0)
  (add `/Game/Game/Widget/BPW_Main.LaucheDice` (`self.WidgetDiceRef`) (delegate `DiceNum`)))

(event `DiceNum`
  (`self.RollTheDice`))

(fn `RollTheDice`
  (locals (Value :type Integer :default 0))
  (bind _output_get (set `local.Value` (`KismetMathLibrary.RandomIntegerInRange` 1 6)))
  (`/Game/Game/BluePrints/BP_Pawn.TryMoving` (`self.Pawn`) _output_get)
  (bind _output_get_2 (set `local.Value` (`KismetMathLibrary.RandomIntegerInRange` 1 20)))
  (`/Game/Game/BluePrints/BP_Hunter.TryMovingHunter` (`self.Hunter`) _output_get_2))

(fn `UserConstructionScript`)