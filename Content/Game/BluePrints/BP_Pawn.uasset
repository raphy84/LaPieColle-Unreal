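; BP_Pawn is the player's board game pawn, which moves between cells and tracks HP (PV).
; HP and cell number live in BP_GameInstance, so BeginPlay restores them, clears the mini-game flag and updates the dice widget.
; TryMoving asks the Board for the next cell, then MoveToCell snaps the pawn there and activates its message.
; ChangePV ignores changes exceeding five and reloads the default level at zero.
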(event `self.ReceiveBeginPlay`
  (bind _as_bp_game_instance (`self.As BP Game Instance`))
  (bind _asbp_game_instance (cast `/Game/Game/Managers/BP_GameInstance` (`GameplayStatics.GetGameInstance`)))
  (bind _output_get (set `self.As BP Game Instance` _asbp_game_instance))
  (bind _playerhp (`/Game/Game/Managers/BP_GameInstance.PlayerHP` _output_get))
  (`/Game/Game/Widget/BPW_Main.UpdatePV` (`/Game/Game/BluePrints/BP_Dice.WidgetDiceRef` (`self.Dice`)) _playerhp)
  (bind _output_get_2 (set `self.PV` _playerhp))
  (if (<= _output_get_2 0)
    (`GameplayStatics.OpenLevelBySoftObjectPtr` "/Game/Game/Levels/DefaultLevel.DefaultLevel")
    (set `/Game/Game/Managers/BP_GameInstance.PlayerHP` 5 _as_bp_game_instance)
    (set `/Game/Game/Managers/BP_GameInstance.CellNumber` 0 _as_bp_game_instance)
    (else
      (bind _asbp_game_instance_2 (cast `/Game/Game/Managers/BP_GameInstance` (`GameplayStatics.GetGameInstance`)))
      (bind _output_get_3 (set `self.Game Instance` _asbp_game_instance_2))
      (`self.MoveToCell`)
      (set `/Game/Game/Managers/BP_GameInstance.InMiniGame` false _output_get_3))))

(fn `ChangePV`
  (params (NexPV :type Integer))
  (if (<= (+ NexPV (`self.PV`)) 5)
    (bind _output_get (set `self.PV` (+ NexPV (`self.PV`))))
    (`/Game/Game/Widget/BPW_Main.UpdatePV` (`/Game/Game/BluePrints/BP_Dice.WidgetDiceRef` (`self.Dice`)) _output_get)
    (set `/Game/Game/Managers/BP_GameInstance.PlayerHP` _output_get (`self.As BP Game Instance`))
    (if (<= _output_get 0)
      (`GameplayStatics.OpenLevelBySoftObjectPtr` "/Game/Game/Levels/DefaultLevel.DefaultLevel")
      (set `/Game/Game/Managers/BP_GameInstance.PlayerHP` 5 (`self.As BP Game Instance`)))))

(fn `MoveToCell`
  (bind _cell (`/Game/Game/BluePrints/BP_Board.GetCellByNumber` (`self.Board`) (`/Game/Game/Managers/BP_GameInstance.CellNumber` (`self.Game Instance`))))
  (bind (_returnvalue_location _returnvalue_rotation) (`KismetMathLibrary.BreakTransform` (`SceneComponent.K2_GetComponentToWorld` (`/Game/Game/BluePrints/Cells/BP_Cell.PawnLocation` _cell))))
  (`self.K2_SetActorLocation` self _returnvalue_location false false)
  (`self.K2_SetActorRotation` self _returnvalue_rotation false)
  (message `/Game/Game/Interfaces/BPI_Interactable.Activate` _cell self))

(fn `TryMoving`
  (params (Value :type Integer))
  (bind _game_instance (`self.Game Instance`))
  (bind _cell (`/Game/Game/BluePrints/BP_Board.GetNextCellToMove` (`self.Board`) (+ Value (`/Game/Game/Managers/BP_GameInstance.CellNumber` _game_instance))))
  (set `/Game/Game/Managers/BP_GameInstance.CellNumber` _cell _game_instance)
  (`self.MoveToCell`))

(fn `UserConstructionScript`)