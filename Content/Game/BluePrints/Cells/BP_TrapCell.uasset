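; BP_TrapCell is a board cell that acts as a one-time trap, costing the pawn that activates it one PV.
; On Activate it calls ChangePV on the pawn, then spawns a plain BP_Cell at its own transform.
; It writes the new cell into its own slot in the BP_Board Cells array and destroys itself.
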(event `/Game/Game/Interfaces/BPI_Interactable.Activate`
  (params (Pawn :type "/Game/Game/BluePrints/BP_Pawn Object Reference"))
  (`/Game/Game/BluePrints/BP_Pawn.ChangePV` Pawn -1)
  (bind _returnvalue (`|SpawnActorFromClass` "/Game/Game/BluePrints/Cells/BP_Cell.BP_Cell_C" (`self.GetTransform`) "AlwaysSpawn" "MultiplyWithRoot" null null))
  (bind _returnvalue_2 (`GameplayStatics.GetActorOfClass` "/Game/Game/BluePrints/BP_Board.BP_Board_C"))
  (bind _cells (`/Game/Game/BluePrints/BP_Board.Cells` _returnvalue_2))
  (`KismetArrayLibrary.Array_Set` _cells (`KismetArrayLibrary.Array_Find` _cells self) _returnvalue true)
  (`self.K2_DestroyActor`))

(fn `UserConstructionScript`
  (`parent.UserConstructionScript`))