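; BP_FoodCelll is a food cell Blueprint that rewards the pawn activating it.
; Its Activate event launches the food dialogue through the widget referenced by the pawn's dice, then calls ChangePV on the pawn with a positive amount.
; BeginPlay, overlap and Tick are disabled stubs, and the construction script only calls its parent.
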(event `/Game/Game/Interfaces/BPI_Interactable.Activate`
  (params (Pawn :type "/Game/Game/BluePrints/BP_Pawn Object Reference"))
  (`/Game/Game/Widget/BPW_Main.LauchDialogue` (`/Game/Game/BluePrints/BP_Dice.WidgetDiceRef` (`/Game/Game/BluePrints/BP_Pawn.Dice` Pawn)) (`self.FoodDialogue`))
  (`/Game/Game/BluePrints/BP_Pawn.ChangePV` Pawn 1))

(fn `UserConstructionScript`
  (`parent.UserConstructionScript`))