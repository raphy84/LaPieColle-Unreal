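; BP_Hunter is the hunter pawn in a dice board game, moving between numbered cells and tracking its HP.
; Each move snaps it to the cell's pawn transform and turns any plain BP_Cell it lands on into a BP_TrapCell, swapped into the board's cell array.
; HP loads from and saves to the GameInstance, ignores changes that would exceed the cap, and triggers the dice widget's victory at zero or below.
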(event `self.ReceiveBeginPlay`
  (bind _asbp_game_instance (cast `/Game/Game/Managers/BP_GameInstance` (`GameplayStatics.GetGameInstance`)))
  (set `self.Game Instance` _asbp_game_instance)
  (set `self.PV` (`/Game/Game/Managers/BP_GameInstance.HunterHP` _asbp_game_instance))
  (`self.MoveToCell` 10))

(event `self.ReceiveTick`
  (params (DeltaSeconds :type "Float (single-precision)")))

(fn `ChangePV`
  (params (NexPV :type Integer))
  (if (<= (+ NexPV (`self.PV`)) 5)
    (bind _output_get (set `self.PV` (+ NexPV (`self.PV`))))
    (set `/Game/Game/Managers/BP_GameInstance.HunterHP` _output_get (`self.Game Instance`))
    (if (<= _output_get 0)
      (`/Game/Game/Widget/BPW_Main.SetVictory` (`/Game/Game/BluePrints/BP_Dice.WidgetDiceRef` (`self.Dice`))))))

(fn `MoveToCell`
  (params (Num :type Integer))
  (bind _cell (`/Game/Game/BluePrints/BP_Board.GetCellByNumber` (`self.Board`) Num))
  (bind (_returnvalue_location _returnvalue_rotation) (`KismetMathLibrary.BreakTransform` (`SceneComponent.K2_GetComponentToWorld` (`/Game/Game/BluePrints/Cells/BP_Cell.PawnLocation` _cell))))
  (`self.K2_SetActorLocation` self _returnvalue_location false false)
  (`self.K2_SetActorRotation` self _returnvalue_rotation false)
  (if (== (`GameplayStatics.GetObjectClass` _cell) "/Game/Game/BluePrints/Cells/BP_Cell.BP_Cell_C")
    (bind _returnvalue (`|SpawnActorFromClass` "/Game/Game/BluePrints/Cells/BP_TrapCell.BP_TrapCell_C" (`self.GetTransform` _cell) "AlwaysSpawn" "MultiplyWithRoot" null null))
    (bind _returnvalue_2 (`GameplayStatics.GetActorOfClass` "/Game/Game/BluePrints/BP_Board.BP_Board_C"))
    (bind _cells (`/Game/Game/BluePrints/BP_Board.Cells` _returnvalue_2))
    (`KismetArrayLibrary.Array_Set` _cells (`KismetArrayLibrary.Array_Find` _cells _cell) _returnvalue true)
    (`self.K2_DestroyActor` _cell)))

(fn `TryMovingHunter`
  (params (Value :type Integer))
  (bind _cell (`/Game/Game/BluePrints/BP_Board.GetNextCellToMove` (`self.Board`) (+ Value (`self.CellNumber`))))
  (bind _output_get (set `self.CellNumber` _cell))
  (`self.MoveToCell` _output_get))

(fn `UserConstructionScript`)